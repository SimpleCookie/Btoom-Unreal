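; Explosion effect actor, a child Blueprint that fires a one-shot physical blast with light and sound, then cleans itself up.
; Shortly after BeginPlay, it fires a radial force impulse and removes the explosion light a moment later.
; In parallel, it plays the explosion sound at the world origin and destroys the actor after a longer delay.
; Its construction script only calls the parent's.
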(event EventBeginPlay
  ;[1 1 1] Comment
  (Utilities|FlowControl|Delay 0.1)
  (Utilities|FlowControl|Sequence
    (:then_0
      (Class|RadialForceComponent|FireImpulse (Variables|Default|GetExplosionRadialForce))
      (Utilities|FlowControl|Delay 0.2)
      (Components|DestroyComponent (Variables|Default|GetExplosionLight)))
    (:then_1
      (Audio|PlaySoundatLocation "/Game/Audio/Explosion01.Explosion01" "0, 0, 0")
      (Utilities|FlowControl|Delay 2.0)
      (Actor|DestroyActor))))

(fn ConstructionScript
  (|CallParentFunction))